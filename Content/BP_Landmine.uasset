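; Landmine actor that flashes when overlapped and, if BP_Erika triggered it, detonates five seconds later.
; A timeline sets the delay of a self-retriggering loop that swaps the mesh between default and emissive materials.
; Detonation runs a debug-drawn sphere trace, spawning a Niagara explosion per processed hit.
; A hit on BP_Erika launches the cached character away by Knockback and destroys the mine.
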(event `StartFlashing`
  (bind (_direction _flashingspeedtrack) (`Timeline|FlashingSpeedTimeline`)
    (:`Update`
      (set `self.ElapsedFlash` _flashingspeedtrack)
      (`self.ChangeMaterial`))))

(event `ChangeMaterial`
  (`KismetSystemLibrary.Delay` (`self.ElapsedFlash`))
  (if (`self.IsFlashing`)
    (`PrimitiveComponent.SetMaterial` (`self.MineMesh`) 0 (`self.DefaultMaterial`))
    (set `self.IsFlashing` false)
    (`self.StartFlashing`)
    (else
      (`PrimitiveComponent.SetMaterial` (`self.MineMesh`) 0 "/Game/Fab/Landmine/M_LandmineEmissive.M_LandmineEmissive")
      (set `self.IsFlashing` true)
      (`self.StartFlashing`))))

(event `self.ReceiveBeginPlay`
  (bind _output_get (set `self.MineLocation` (`self.K2_GetActorLocation`)))
  (set `self.DefaultMaterial` (`PrimitiveComponent.GetMaterial` (`self.MineMesh`) 0))
  (set `self.IsFlashing` false))

(event `self.MineCollision.OnComponentBeginOverlap`
  (params (OverlappedComponent :type "PrimitiveComponent Object Reference") (OtherActor :type "Actor Object Reference") (OtherComp :type "PrimitiveComponent Object Reference") (OtherBodyIndex :type Integer) (bFromSweep :type Boolean) (SweepResult :type "HitResult Structure (by ref)"))
  (bind _minelocation (`self.MineLocation`))
  (`self.StartFlashing`)
  (bind _asbp_erika (cast `/Game/MyCharacters/Erika/ErikaStuff/BP_Erika` OtherActor))
  (set `self.As BP Erika` _asbp_erika)
  (`KismetSystemLibrary.Delay` 5.0)
  (bind (_outhits _returnvalue) (`KismetSystemLibrary.SphereTraceMulti` :`Start` (stale `self.ReceiveBeginPlay` _output_get) :`End` (stale `self.ReceiveBeginPlay` _output_get) :`Radius` 500.0 :`TraceChannel` "TraceTypeQuery1" :`DrawDebugType` "ForDuration" :`DrawTime` 10.0))
  (if _returnvalue
    (for _array_element _outhits
      (`NiagaraFunctionLibrary.SpawnSystemAtLocation` "/Game/MsvFx_Niagara_Explosion_Pack_01/Prefabs/Niagara_Dust_Explosion_01.Niagara_Dust_Explosion_01" _minelocation (`KismetMathLibrary.Conv_VectorToRotator` _minelocation))
      (bind (_bblockinghit _binitialoverlap _time _distance _location _impactpoint _normal _impactnormal _physmat _hitactor _hitcomponent _hitbonename _bonename _hititem _elementindex _faceindex _tracestart _traceend) (`GameplayStatics.BreakHitResult` _array_element))
      (bind _asbp_erika_2 (cast `/Game/MyCharacters/Erika/ErikaStuff/BP_Erika` _hitactor))
      (bind _returnvalue_2 (`KismetSystemLibrary.GetDisplayName` _asbp_erika_2))
      (`KismetSystemLibrary.PrintString` _returnvalue_2 true true (struct :`G` 0.66 :`B` 1.0 :`A` 1.0) 10.0 (`KismetStringLibrary.Conv_StringToName` _returnvalue_2))
      (`Character.LaunchCharacter` (`self.As BP Erika`) (* (`KismetMathLibrary.Normal` (- (`self.K2_GetActorLocation` (`self.As BP Erika`)) _traceend)) (`self.Knockback`)) false false)
      (`self.K2_DestroyActor`))))

(fn `UserConstructionScript`)