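; BP_CompassSimple is a simple compass that prints which cardinal direction the player character faces.
; BeginPlay defines fixed North (-Y) and East (+X) world vectors.
; Each Tick dots the player's forward vector with both, negates the results for South and West, and prints whichever direction's helper check finds strictly largest.
; Exact ties print nothing.
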(event `self.ReceiveTick`
  (params (DeltaSeconds :type "Float (single-precision)"))
  (bind _returnvalue (`self.GetActorForwardVector` (`GameplayStatics.GetPlayerCharacter` 0)))
  (set `self.DotNorth` (`KismetMathLibrary.Dot_VectorVector` _returnvalue (`self.NorthVector`)))
  (set `self.DotEast` (`KismetMathLibrary.Dot_VectorVector` _returnvalue (`self.EastVector`)))
  (set `self.DotSouth` (* (`self.DotNorth`) -1.0))
  (set `self.DotWest` (* (`self.DotEast`) -1.0))
  (bind _returnvalue_2 (`self.IsNorth`))
  (if _returnvalue_2
    (`KismetSystemLibrary.PrintString` "North" true true (struct :`G` 0.66 :`B` 1.0 :`A` 1.0) 0.5 "North")
    (else
      (bind _returnvalue_3 (`self.IsEast`))
      (if _returnvalue_3
        (`KismetSystemLibrary.PrintString` "East" true true (struct :`G` 0.66 :`B` 1.0 :`A` 1.0) 0.5 "East")
        (else
          (bind _returnvalue_4 (`self.IsSouth`))
          (if _returnvalue_4
            (`KismetSystemLibrary.PrintString` "South" true true (struct :`G` 0.66 :`B` 1.0 :`A` 1.0) 0.5 "South")
            (else
              (bind _returnvalue_5 (`self.IsWest`))
              (if _returnvalue_5
                (`KismetSystemLibrary.PrintString` "West" true true (struct :`G` 0.66 :`B` 1.0 :`A` 1.0) 0.5 "West")))))))))

(event `self.ReceiveBeginPlay`
  (set `self.NorthVector` (`KismetMathLibrary.MakeVector` 0.0 -1.0))
  (set `self.EastVector` (`KismetMathLibrary.MakeVector` 1.0)))

(fn `IsEast`
  (returns (ReturnValue :type Boolean))
  (return (and (and (> (`self.DotEast`) (`self.DotNorth`)) (> (`self.DotEast`) (`self.DotSouth`))) (> (`self.DotEast`) (`self.DotWest`)))))

(fn `IsNorth`
  (returns (ReturnValue :type Boolean))
  (return (and (and (> (`self.DotNorth`) (`self.DotEast`)) (> (`self.DotNorth`) (`self.DotSouth`))) (> (`self.DotNorth`) (`self.DotWest`)))))

(fn `IsSouth`
  (returns (ReturnValue :type Boolean))
  (return (and (and (> (`self.DotSouth`) (`self.DotNorth`)) (> (`self.DotSouth`) (`self.DotEast`))) (> (`self.DotSouth`) (`self.DotWest`)))))

(fn `IsWest`
  (returns (ReturnValue :type Boolean))
  (return (and (and (> (`self.DotWest`) (`self.DotEast`)) (> (`self.DotWest`) (`self.DotSouth`))) (> (`self.DotWest`) (`self.DotNorth`)))))

(fn `UserConstructionScript`)