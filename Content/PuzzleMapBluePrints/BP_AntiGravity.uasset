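; BP_AntiGravity is a volume that pushes a BP_PickupObject upward while it is inside.
; Overlap events on CollisionComponent store the pickup and track whether one is present.
; Each tick, if one is present and Activated is set, it applies an upward force to the object's mesh, scaled by ForceStrength.
; It tracks a single pickup, and nothing in these graphs sets Activated.
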(event `self.CollisionComponent.OnComponentBeginOverlap`
  (params (OverlappedComponent :type "PrimitiveComponent Object Reference") (OtherActor :type "Actor Object Reference") (OtherComp :type "PrimitiveComponent Object Reference") (OtherBodyIndex :type Integer) (bFromSweep :type Boolean) (SweepResult :type "HitResult Structure (by ref)"))
  (bind _asbp_pickup_object (cast `/Game/PuzzleMapBluePrints/BP_PickupObject` OtherActor))
  (set `self.PickupRef` _asbp_pickup_object)
  (set `self.IsObjectIn` true))

(event `self.CollisionComponent.OnComponentEndOverlap`
  (params (OverlappedComponent :type "PrimitiveComponent Object Reference") (OtherActor :type "Actor Object Reference") (OtherComp :type "PrimitiveComponent Object Reference") (OtherBodyIndex :type Integer))
  (cast `/Game/PuzzleMapBluePrints/BP_PickupObject` OtherActor)
  (set `self.IsObjectIn` false))

(event `self.ReceiveTick`
  (params (DeltaSeconds :type "Float (single-precision)"))
  (if (`self.IsObjectIn`)
    (if (`self.Activated`)
      (`PrimitiveComponent.AddForce` (`/Game/PuzzleMapBluePrints/BP_PickupObject.ObjectMesh` (`self.PickupRef`)) (* (0.0 0.0 100.0) (`self.ForceStrength`)) "None" false))))

(fn `UserConstructionScript`)