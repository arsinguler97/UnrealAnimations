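; BP_PickupObject is a puzzle-map pickup object that comes in Red, Blue and Green variants, chosen by its ObjectID.
; The construction script switches on the ObjectID as a string, giving each variant its own static mesh and setting the matching Base Color vector parameter on the mesh materials.
; The file holds only this visual setup, with no pickup or interaction logic.
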(fn `UserConstructionScript`
  (bind _objectmesh (`self.ObjectMesh`))
  (bind _objectmesh_2 (`self.ObjectMesh`))
  (switch `string` (`KismetStringLibrary.Conv_NameToString` (`self.ObjectID`))
    (:`Red`
      (`StaticMeshComponent.SetStaticMesh` _objectmesh_2 "/Game/Fab/PickupObject/prism.prism")
      (`MeshComponent.SetVectorParameterValueOnMaterials` _objectmesh "Base Color" (1.0 0.0 0.0)))
    (:`Blue`
      (`StaticMeshComponent.SetStaticMesh` _objectmesh_2 "/Game/Fab/PickupObject/Sci-Fi-Cube.Sci-Fi-Cube")
      (`MeshComponent.SetVectorParameterValueOnMaterials` _objectmesh "Base Color" (0.0 0.0 1.0)))
    (:`Green`
      (`StaticMeshComponent.SetStaticMesh` _objectmesh_2 "/Game/Fab/PickupObject/robo-orb_sculpt.robo-orb_sculpt")
      (`MeshComponent.SetVectorParameterValueOnMaterials` _objectmesh "Base Color" (0.0 1.0 0.0)))))