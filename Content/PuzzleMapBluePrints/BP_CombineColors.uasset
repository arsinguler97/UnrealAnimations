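; Puzzle machine that merges two pickup objects of different colors into one cube of their blended color.
; Its overlap volume tracks tagged pickups; with two or more inside, a timeline lowers the mesh, working audio plays, then the mesh rises after combining.
; The first two pickups' material colors are averaged for a spawned replacement, always given ObjectID "Purple".
; Matching colors instead play an error sound and leave both objects intact.
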(event `self.CombineColorsCollision.OnComponentBeginOverlap`
  (params (OverlappedComponent :type "PrimitiveComponent Object Reference") (OtherActor :type "Actor Object Reference") (OtherComp :type "PrimitiveComponent Object Reference") (OtherBodyIndex :type Integer) (bFromSweep :type Boolean) (SweepResult :type "HitResult Structure (by ref)"))
  (if (`self.ActorHasTag` OtherActor "PickupObject")
    (bind _asbp_pickup_object (cast `/Game/PuzzleMapBluePrints/BP_PickupObject` OtherActor))
    (`KismetArrayLibrary.Array_Add` (`self.Pickups`) _asbp_pickup_object)
    (if (and (not (`self.CombiningColors`)) (>= (`KismetArrayLibrary.Array_Length` (`self.Pickups`)) 2))
      (`KismetSystemLibrary.Delay` 1.0)
      (`self.CombineClose`)
      (`AudioComponent.Play` (`self.Working`) 0.0)
      (`KismetSystemLibrary.Delay` 2.0)
      (`self.StartToCombine`)
      (`AudioComponent.Stop` (`self.Working`))
      (`KismetSystemLibrary.Delay` 0.2)
      (`self.CombineOpen`))))

(event `self.CombineColorsCollision.OnComponentEndOverlap`
  (params (OverlappedComponent :type "PrimitiveComponent Object Reference") (OtherActor :type "Actor Object Reference") (OtherComp :type "PrimitiveComponent Object Reference") (OtherBodyIndex :type Integer))
  (if (`self.ActorHasTag` OtherActor "PickupObject")
    (bind _asbp_pickup_object (cast `/Game/PuzzleMapBluePrints/BP_PickupObject` OtherActor))
    (`KismetArrayLibrary.Array_RemoveItem` (`self.Pickups`) _asbp_pickup_object)))

(event `StartToCombine`
  (bind _spawnpoint (`self.SpawnPoint`))
  (set `self.CombiningColors` true)
  (set `self.ObjectA` (`|GetArrayItem` (`self.Pickups`)))
  (set `self.ObjectB` (`|GetArrayItem` (`self.Pickups`) 1))
  (bind _asmaterial_instance_dynamic (cast `MaterialInstanceDynamic` (`PrimitiveComponent.GetMaterial` (`/Game/PuzzleMapBluePrints/BP_PickupObject.ObjectMesh` (`self.ObjectA`)) 0)))
  (bind _returnvalue (`MaterialInstanceDynamic.K2_GetVectorParameterValue` _asmaterial_instance_dynamic "Base Color"))
  (set `self.ObjectAParameters` _returnvalue)
  (bind _asmaterial_instance_dynamic_2 (cast `MaterialInstanceDynamic` (`PrimitiveComponent.GetMaterial` (`/Game/PuzzleMapBluePrints/BP_PickupObject.ObjectMesh` (`self.ObjectB`)) 0)))
  (bind _returnvalue_2 (`MaterialInstanceDynamic.K2_GetVectorParameterValue` _asmaterial_instance_dynamic_2 "Base Color"))
  (set `self.ObjectBParameters` _returnvalue_2)
  (if (== (`self.ObjectAParameters`) (`self.ObjectBParameters`))
    (set `self.CombiningColors` false)
    (`GameplayStatics.PlaySoundAtLocation` "/Game/Audio/Wrong.Wrong" (`self.K2_GetActorLocation` self) (struct) 1.0 1.0 0.0 null null null null)
    (else
      (`self.K2_DestroyActor` (`self.ObjectA`))
      (`self.K2_DestroyActor` (`self.ObjectB`))
      (`self.NewColor`)
      (bind _returnvalue_3 (`|SpawnActorFromClass` "/Game/PuzzleMapBluePrints/BP_PickupObject.BP_PickupObject_C" (`KismetMathLibrary.MakeTransform` (`SceneComponent.K2_GetComponentLocation` _spawnpoint) (`SceneComponent.K2_GetComponentRotation` _spawnpoint)) "AlwaysSpawn" "MultiplyWithRoot" null "Purple" null null))
      (bind _output_get (set `self.NewObject` _returnvalue_3))
      (`StaticMeshComponent.SetStaticMesh` (`/Game/PuzzleMapBluePrints/BP_PickupObject.ObjectMesh` _output_get) "/Game/Fab/PickupObject/Sci-Fi-Cube.Sci-Fi-Cube")
      (bind _returnvalue_4 (`PrimitiveComponent.CreateDynamicMaterialInstance` (`/Game/PuzzleMapBluePrints/BP_PickupObject.ObjectMesh` _output_get) 0 "/Game/LevelPrototyping/Materials/M_Solid.M_Solid" "None"))
      (`MaterialInstanceDynamic.SetVectorParameterValue` _returnvalue_4 "Base Color" (`self.NewCombinedColor`))
      (set `self.CombiningColors` false))))

(event `self.ReceiveBeginPlay`
  (bind _output_get (set `self.CombineColorsStart` (`self.K2_GetActorLocation`)))
  (set `self.CombineColorsEnd` (+ _output_get (0.0 0.0 -800.0))))

(event `CombineClose`
  (bind (_direction _newtrack_0) (`Timeline|CombineDoor` :!label _label)
    (:`Update`
      (`SceneComponent.K2_SetWorldLocation` (`self.CombineColorsMesh`) (`KismetMathLibrary.VLerp` (`self.CombineColorsStart`) (`self.CombineColorsEnd`) _newtrack_0) false false))))

(event `CombineOpen`
  (goto _label :!via `Reverse`))

(fn `NewColor`
  (bind (_objectaparameters_r _objectaparameters_g _objectaparameters_b) (break `LinearColor` (`self.ObjectAParameters`)))
  (bind (_objectbparameters_r _objectbparameters_g _objectbparameters_b) (break `LinearColor` (`self.ObjectBParameters`)))
  (set `self.NewCombinedColor` (make `LinearColor` (/ (+ _objectaparameters_r _objectbparameters_r) 2.0) (/ (+ _objectaparameters_g _objectbparameters_g) 2.0) (/ (+ _objectaparameters_b _objectbparameters_b) 2.0) 1.0)))

(fn `UserConstructionScript`)