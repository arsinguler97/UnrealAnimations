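; BP_Door is a color-coded puzzle-map door that slides straight up to open and back down to close.
; On BeginPlay it caches its start position and an end point above it; OpenDoor plays the DoorMove timeline to lerp between them, and CloseDoor reverses it, both updating a DoorOpen flag.
; The construction script tints the mesh red, blue or green from DoorID, so the color previews in the editor.
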(event `self.ReceiveBeginPlay`
  (bind _output_get (set `self.DoorStart` (`self.K2_GetActorLocation`)))
  (set `self.DoorEnd` (+ _output_get (0.0 0.0 400.0))))

(event `OpenDoor`
  (set `self.DoorOpen` true)
  (bind (_direction _newtrack_0) (`Timeline|DoorMove` :!label _label)
    (:`Update`
      (`self.K2_SetActorLocation` (`KismetMathLibrary.VLerp` (`self.DoorStart`) (`self.DoorEnd`) _newtrack_0)))))

(event `CloseDoor`
  (set `self.DoorOpen` false)
  (goto _label :!via `Reverse`))

(fn `UserConstructionScript`
  (bind _staticmesh (`self.StaticMesh`))
  (switch `string` (`KismetStringLibrary.Conv_NameToString` (`self.DoorID`))
    (:`Red`
      (`MeshComponent.SetVectorParameterValueOnMaterials` _staticmesh "Base Color" (1.0 0.0 0.0)))
    (:`Blue`
      (`MeshComponent.SetVectorParameterValueOnMaterials` _staticmesh "Base Color" (0.0 0.0 1.0)))
    (:`Green`
      (`MeshComponent.SetVectorParameterValueOnMaterials` _staticmesh "Base Color" (0.0 1.0 0.0)))))