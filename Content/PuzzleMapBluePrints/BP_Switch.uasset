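; BP_Switch is a puzzle map switch that turns a BP_AntiGravity actor on and off.
; On BeginPlay it caches a reference to that actor through GetActorOfClass.
; Every Tick it polls the visibility of StaticMeshOn, copies that state to the actor's Activated flag and calls PlaySound or StopSound to match.
; Nothing in its graphs changes the mesh visibility.
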(event `self.ReceiveBeginPlay`
  (bind _returnvalue (`GameplayStatics.GetActorOfClass` "/Game/PuzzleMapBluePrints/BP_AntiGravity.BP_AntiGravity_C"))
  (set `self.AntiGravityRef` _returnvalue))

(event `self.ReceiveTick`
  (params (DeltaSeconds :type "Float (single-precision)"))
  (bind _antigravityref (`self.AntiGravityRef`))
  (if (`SceneComponent.IsVisible` (`self.StaticMeshOn`))
    (set `/Game/PuzzleMapBluePrints/BP_AntiGravity.Activated` true _antigravityref)
    (`/Game/PuzzleMapBluePrints/BP_AntiGravity.PlaySound` _antigravityref)
    (else
      (set `/Game/PuzzleMapBluePrints/BP_AntiGravity.Activated` false _antigravityref)
      (`/Game/PuzzleMapBluePrints/BP_AntiGravity.StopSound` _antigravityref))))

(fn `UserConstructionScript`)