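; Puzzle combine box that merges two differently colored pickup objects into one of the third color among Red, Green and Blue.
; Overlap events track tagged pickups; with two inside, a timeline lowers the box mesh, then raises it after combining.
; Combining matches material display names, spawns a recolored pickup with a new ID, destroys both originals and plays a Niagara burst.
; Matching colors are left uncombined.
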(event `self.CombineBoxCollision.OnComponentBeginOverlap`
  (params (OverlappedComponent :type "PrimitiveComponent Object Reference") (OtherActor :type "Actor Object Reference") (OtherComp :type "PrimitiveComponent Object Reference") (OtherBodyIndex :type Integer) (bFromSweep :type Boolean) (SweepResult :type "HitResult Structure (by ref)"))
  (if (`self.ActorHasTag` OtherActor "PickupObject")
    (bind _asbp_pickup_object (cast `/Game/PuzzleMapBluePrints/BP_PickupObject` OtherActor))
    (`KismetArrayLibrary.Array_Add` (`self.PickupList`) _asbp_pickup_object)
    (if (and (not (`self.IsProcessing`)) (>= (`KismetArrayLibrary.Array_Length` (`self.PickupList`)) 2))
      (`KismetSystemLibrary.PrintString` "Dogru")
      (`KismetSystemLibrary.Delay` 0.5)
      (`self.CombineClose`)
      (`KismetSystemLibrary.Delay` 4.0)
      (`self.StartCombine`)
      (`KismetSystemLibrary.PrintString` (`self.CombinedName`))
      (`KismetSystemLibrary.Delay` 0.2)
      (`self.CombineOpen`))))

(event `self.CombineBoxCollision.OnComponentEndOverlap`
  (params (OverlappedComponent :type "PrimitiveComponent Object Reference") (OtherActor :type "Actor Object Reference") (OtherComp :type "PrimitiveComponent Object Reference") (OtherBodyIndex :type Integer))
  (if (`self.ActorHasTag` OtherActor "PickupObject")
    (bind _asbp_pickup_object (cast `/Game/PuzzleMapBluePrints/BP_PickupObject` OtherActor))
    (`KismetArrayLibrary.Array_RemoveItem` (`self.PickupList`) _asbp_pickup_object)))

(event `StartCombine`
  (bind _newpickupobject (`self.NewPickupObject`))
  (set `self.IsProcessing` true)
  (set `self.PickupA` (`|GetArrayItem` (`self.PickupList`)))
  (set `self.PickupB` (`|GetArrayItem` (`self.PickupList`) 1))
  (set `self.MaterialA` (`KismetSystemLibrary.GetDisplayName` (`PrimitiveComponent.GetMaterial` (`/Game/PuzzleMapBluePrints/BP_PickupObject.ObjectMesh` (`self.PickupA`)) 0)))
  (set `self.MaterialB` (`KismetSystemLibrary.GetDisplayName` (`PrimitiveComponent.GetMaterial` (`/Game/PuzzleMapBluePrints/BP_PickupObject.ObjectMesh` (`self.PickupB`)) 0)))
  (if (== (`self.MaterialA`) (`self.MaterialB`))
    (set `self.IsProcessing` false)
    (else
      (`self.CombineNames`)
      (bind _returnvalue (`|SpawnActorFromClass` "/Game/PuzzleMapBluePrints/BP_PickupObject.BP_PickupObject_C" (`KismetMathLibrary.MakeTransform` (`SceneComponent.K2_GetComponentLocation` (`self.SpawnPoint`)) (`SceneComponent.K2_GetComponentRotation` (`self.SpawnPoint`))) "AlwaysSpawn" "MultiplyWithRoot" null "None" null null))
      (set `self.NewPickupObject` _returnvalue)
      (`PrimitiveComponent.SetMaterial` (`/Game/PuzzleMapBluePrints/BP_PickupObject.ObjectMesh` _newpickupobject) 0 (`BlueprintMapLibrary.Map_Find` (`self.MaterialMap`) (`self.CombinedName`)))
      (set `/Game/PuzzleMapBluePrints/BP_PickupObject.ObjectID` (`KismetStringLibrary.Conv_StringToName` (`KismetStringLibrary.Concat_StrStr` "Combined" (`self.CombinedName`))) _newpickupobject)
      (`self.K2_DestroyActor` (`self.PickupA`))
      (`self.K2_DestroyActor` (`self.PickupB`))
      (`KismetArrayLibrary.Array_Clear` (`self.PickupList`))
      (`NiagaraFunctionLibrary.SpawnSystemAtLocation` "/Game/Pack_Simple_Particle_Burst/01_Niagara_Systems/NS_Simple_Burst_Level_3.NS_Simple_Burst_Level_3" (`SceneComponent.K2_GetComponentLocation` (`self.Scene`)))
      (set `self.IsProcessing` false))))

(event `self.ReceiveBeginPlay`
  (bind _output_get (set `self.CombineDoorStart` (`self.K2_GetActorLocation`)))
  (set `self.CombineDoorEnd` (+ _output_get (0.0 0.0 -600.0))))

(event `CombineClose`
  (bind (_direction _newtrack_0) (`Timeline|CombineDoor` :!label _label)
    (:`Update`
      (`SceneComponent.K2_SetWorldLocation` (`self.CombineBoxMesh`) (`KismetMathLibrary.VLerp` (`self.CombineDoorStart`) (`self.CombineDoorEnd`) _newtrack_0) false false))))

(event `CombineOpen`
  (goto _label :!via `Reverse`))

(fn `CombineNames`
  (switch `string` (`self.MaterialA`)
    (:`Red`
      (if (== (`self.MaterialB`) "Blue")
        (set `self.CombinedName` "Green")
        (else
          (set `self.CombinedName` "Blue"))))
    (:`Blue`
      (if (== (`self.MaterialB`) "Red")
        (set `self.CombinedName` "Green")
        (else
          (set `self.CombinedName` "Red"))))
    (:`Green`
      (if (== (`self.MaterialB`) "Blue")
        (set `self.CombinedName` "Red")
        (else
          (set `self.CombinedName` "Blue"))))))

(fn `UserConstructionScript`)