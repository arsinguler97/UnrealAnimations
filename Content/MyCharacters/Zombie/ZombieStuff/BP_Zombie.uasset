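; BP_Zombie is an AI enemy character that attacks the player and tints its emissive material red, blue or green by color ID.
; BeginPlay hands AI_Zombie a player target (Erika, else first-person character) and a pickup object.
; A looping timer deals damage while attacking within range.
; TakeDamage flags the blackboard and marks death, which another polling timer turns into a halt and delayed destroy.
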(event `self.ReceiveBeginPlay`
  (bind _returnvalue (`self.GetController`))
  (`|ExecutionSequence`
    (:`then_0`
      (bind _returnvalue_2 (`GameplayStatics.GetActorOfClass` "/Game/MyCharacters/Erika/ErikaStuff/BP_Erika.BP_Erika_C"))
      (set `self.PlayerCharacter` _returnvalue_2)
      (bind _returnvalue_3 (`GameplayStatics.GetActorOfClass` "/Game/PuzzleMapBluePrints/BP_PickupObject.BP_PickupObject_C"))
      (set `self.PickupObjectRef` _returnvalue_3)
      (bind _returnvalue_4 (`GameplayStatics.GetActorOfClass` "/Game/FirstPerson/Blueprints/BP_FirstPersonCharacter.BP_FirstPersonCharacter_C"))
      (set `self.FirstPersonRef` _returnvalue_4))
    (:`then_1`
      (bind _asai_zombie (cast `/Game/MyCharacters/Zombie/AI_Zombie` _returnvalue))
      (bind _playercharacter (`self.PlayerCharacter`)
        (:`then`
          (`/Game/MyCharacters/Zombie/AI_Zombie.SetPlayerTarget` _asai_zombie _playercharacter null))
        (:`else`
          (`/Game/MyCharacters/Zombie/AI_Zombie.SetPlayerTarget` _asai_zombie null (`self.FirstPersonRef`)))))
    (:`then_2`
      (bind _asai_zombie_2 (cast `/Game/MyCharacters/Zombie/AI_Zombie` _returnvalue))
      (`/Game/MyCharacters/Zombie/AI_Zombie.SetPickupTarget` _asai_zombie_2 (`self.PickupObjectRef`)))
    (:`then_3`
      (`KismetSystemLibrary.K2_SetTimer` null "DealDamage" 0.25 true))
    (:`then_4`
      ; DestroyZombie
      (`KismetSystemLibrary.K2_SetTimerDelegate` (delegate `DestoryZombie`) 1.0 true))))

(event `DestoryZombie`
  ; DestroyZombie
  (if (`self.IsDead`)
    (set `CharacterMovementComponent.MaxWalkSpeed` 0.0 (`self.CharacterMovement`))
    (`KismetSystemLibrary.Delay` 3.333333)
    (`self.K2_DestroyActor`)))

(fn `DealDamage`
  (if (`self.IsZombieAttacking`)
    (if (<= (`self.DistanceToPlayer`) (`self.DamageRange`))
      (bind _playercharacter (`self.PlayerCharacter`)
        (:`then`
          (`/Game/MyCharacters/Erika/ErikaStuff/BP_Erika.PlayerTakeDamage` _playercharacter))
        (:`else`
          (`/Game/FirstPerson/Blueprints/BP_FirstPersonCharacter.FirstPersonTakeDamage` (`self.FirstPersonRef`)))))))

(fn `DistanceToPlayer`
  (returns (ReturnValue :type "Float (double-precision)"))
  (return (`KismetMathLibrary.Vector_Distance` (`self.K2_GetActorLocation` self) (`self.K2_GetActorLocation` (`GameplayStatics.GetPlayerCharacter` 0)))))

(fn `TakeDamage`
  (params (DamageAmount :type "Float (double-precision)"))
  (bind _asai_zombie (cast `/Game/MyCharacters/Zombie/AI_Zombie` (`self.GetController`)))
  (`BlackboardComponent.SetValueAsBool` (`AIController.Blackboard` _asai_zombie) "GotHit" true)
  (set `self.CurrentHealth` (`KismetMathLibrary.FClamp` (- (`self.CurrentHealth`) DamageAmount) 0.0 (`self.MaxHealth`)))
  (if (<= (`self.CurrentHealth`) 0.0)
    (set `self.IsDead` true)))

(fn `UserConstructionScript`
  (bind _mesh (`self.Mesh`))
  (switch `string` (`KismetStringLibrary.Conv_NameToString` (`self.ZombieColorID`))
    (:`Red`
      (`MeshComponent.SetVectorParameterValueOnMaterials` _mesh "EmissiveParameter" (1.0 0.0 0.0)))
    (:`Blue`
      (`MeshComponent.SetVectorParameterValueOnMaterials` _mesh "EmissiveParameter" (0.0 0.0 1.0)))
    (:`Green`
      (`MeshComponent.SetVectorParameterValueOnMaterials` _mesh "EmissiveParameter" (0.0 1.0 0.0)))))